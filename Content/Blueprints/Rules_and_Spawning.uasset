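; Rules and spawning Blueprint that builds a fixed, branching corridor map, Map001, on BeginPlay from modular actor pieces.
; Helper functions spawn straight pieces, turns, side halls, 3-way and 4-way junctions, each returning the new actor's exit transforms.
; Map001 hard-codes the layout by feeding each exit into the next spawn, with nested Sequence nodes handling branches and Stairs placed at two points.
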(event EventBeginPlay
  (CallFunction|Map001))

(fn ConstructionScript)

(fn SpawnMapPiece
  (params (Spawn%20Point :type Transform))
  (bind _returnvalue (Game|SpawnActorfromClass "/Game/Blueprints/Map_Pieces/Main.Main_C" (Math|Transform|SelectTransform Spawn%20Point (Variables|Default|GetspawnPoint) (Variables|Default|GetPick%20A)) "Undefined" 0 0))
  (bind _spawnpoint (Default|GetSpawnPoint _returnvalue))
  (bind _output_get (Variables|Default|SetspawnPoint _spawnpoint))
  (return _output_get))

(fn Map001
  (bind _current_spawn_point (CallFunction|SpawnMapPiece (Variables|Default|GetspawnPoint)))
  (Game|SpawnActorfromClass "/Game/Blueprints/Map_Pieces/Stairs.Stairs_C" (Math|Transform|MakeTransform "0, 0, 0" "0,180.000000, 0") "Undefined" 0 0)
  (bind _current_spawn_point_2 (CallFunction|SpawnMapPiece _current_spawn_point))
  (bind _current_spawn_point_3 (CallFunction|SpawnMapPiece _current_spawn_point_2))
  (bind _foward_spawn_point (CallFunction|SpawnRightHall _current_spawn_point_3))
  (bind _left_spawn_point (CallFunction|SpawnLeftTurn _foward_spawn_point))
  (bind _left_spawn_point_2 (CallFunction|SpawnLeftTurn _left_spawn_point))
  (bind _current_spawn_point_4 (CallFunction|SpawnMapPiece _left_spawn_point_2))
  (bind _right_spawn_point (CallFunction|SpawnRightTurn _current_spawn_point_4))
  (bind _current_spawn_point_5 (CallFunction|SpawnMapPiece _right_spawn_point))
  (bind _foward_spawn_point_2 (CallFunction|SpawnRightHall _current_spawn_point_5))
  (bind _current_spawn_point_6 (CallFunction|SpawnMapPiece _foward_spawn_point_2))
  (bind _current_spawn_point_7 (CallFunction|SpawnMapPiece _current_spawn_point_6))
  (bind _current_spawn_point_8 (CallFunction|SpawnMapPiece _current_spawn_point_7))
  (bind _right_spawn_point_2 (CallFunction|SpawnRightTurn _current_spawn_point_8))
  (bind _current_spawn_point_9 (CallFunction|SpawnMapPiece _right_spawn_point_2))
  (bind _right_spawn_point_3 (CallFunction|SpawnRightTurn _current_spawn_point_9))
  (bind _current_spawn_point_10 (CallFunction|SpawnMapPiece _right_spawn_point_3))
  (bind (_foward_spawn_point_3 _left_spawn_point_3) (CallFunction|SpawnLeftHall _current_spawn_point_10))
  (Utilities|FlowControl|Sequence
    (:then_0
      (bind _current_spawn_point_11 (CallFunction|SpawnMapPiece _foward_spawn_point_3))
      (bind (_left_spawn_point_4 _right_spawn_point_4) (CallFunction|Spawn3-way _current_spawn_point_11))
      (CallFunction|SpawnMapPiece _right_spawn_point_4)
      (bind _current_spawn_point_12 (CallFunction|SpawnMapPiece _left_spawn_point_4))
      (bind _current_spawn_point_13 (CallFunction|SpawnMapPiece _current_spawn_point_12))
      (bind _left_spawn_point_5 (CallFunction|SpawnLeftTurn _current_spawn_point_13))
      (CallFunction|SpawnMapPiece _left_spawn_point_5))
    (:then_1
      (bind _current_spawn_point_14 (CallFunction|SpawnMapPiece _left_spawn_point_3))
      (bind _current_spawn_point_15 (CallFunction|SpawnMapPiece _current_spawn_point_14))
      (bind _foward_spawn_point_4 (CallFunction|SpawnRightHall _current_spawn_point_15))
      (bind _current_spawn_point_16 (CallFunction|SpawnMapPiece _foward_spawn_point_4))
      (bind _right_spawn_point_5 (CallFunction|SpawnRightTurn _current_spawn_point_16))
      (bind _current_spawn_point_17 (CallFunction|SpawnMapPiece _right_spawn_point_5))
      (bind _left_spawn_point_6 (CallFunction|SpawnLeftTurn _current_spawn_point_17))
      (bind (_right_spawn_point_6 _foward_spawn_point_5) (CallFunction|SpawnRightHall _left_spawn_point_6))
      (Utilities|FlowControl|Sequence
        (:then_0
          (Game|SpawnActorfromClass "/Game/Blueprints/Map_Pieces/Stairs.Stairs_C" _foward_spawn_point_5 "Undefined" 0 0))
        (:then_1
          (bind _current_spawn_point_18 (CallFunction|SpawnMapPiece _right_spawn_point_6))
          (bind (_right_spawn_point_7 _foward_spawn_point_6) (CallFunction|SpawnRightHall _current_spawn_point_18))
          (Utilities|FlowControl|Sequence
            (:then_0
              (bind _current_spawn_point_19 (CallFunction|SpawnMapPiece _right_spawn_point_7))
              (bind _left_spawn_point_7 (CallFunction|SpawnLeftTurn _current_spawn_point_19))
              (CallFunction|SpawnMapPiece _left_spawn_point_7))
            (:then_1
              (bind _current_spawn_point_20 (CallFunction|SpawnMapPiece _foward_spawn_point_6))
              (bind (_right_spawn_point_8 _foward_spawn_point_7) (CallFunction|SpawnRightHall _current_spawn_point_20))
              (Utilities|FlowControl|Sequence
                (:then_0
                  (bind _current_spawn_point_21 (CallFunction|SpawnMapPiece _right_spawn_point_8))
                  (bind (_left_spawn_point_8 _right_spawn_point_9 _foward_spawn_point_8) (CallFunction|Spawn4-way _current_spawn_point_21))
                  (bind _current_spawn_point_22 (CallFunction|SpawnMapPiece _left_spawn_point_8))
                  (CallFunction|SpawnMapPiece _current_spawn_point_22)
                  (bind _current_spawn_point_23 (CallFunction|SpawnMapPiece _foward_spawn_point_8))
                  (bind _left_spawn_point_9 (CallFunction|SpawnLeftTurn _current_spawn_point_23))
                  (bind _right_spawn_point_10 (CallFunction|SpawnRightTurn _left_spawn_point_9))
                  (bind _current_spawn_point_24 (CallFunction|SpawnMapPiece _right_spawn_point_10))
                  (bind _current_spawn_point_25 (CallFunction|SpawnMapPiece _current_spawn_point_24))
                  (bind (_right_spawn_point_11 _foward_spawn_point_9) (CallFunction|SpawnRightHall _current_spawn_point_25))
                  (CallFunction|SpawnMapPiece _right_spawn_point_11)
                  (bind _foward_spawn_point_10 (CallFunction|SpawnLeftHall _foward_spawn_point_9))
                  (bind _current_spawn_point_26 (CallFunction|SpawnMapPiece _foward_spawn_point_10))
                  (bind _left_spawn_point_10 (CallFunction|SpawnLeftTurn _current_spawn_point_26))
                  (bind _current_spawn_point_27 (CallFunction|SpawnMapPiece _left_spawn_point_10))
                  (bind _left_spawn_point_11 (CallFunction|SpawnLeftTurn _current_spawn_point_27))
                  (bind _current_spawn_point_28 (CallFunction|SpawnMapPiece _left_spawn_point_11))
                  (bind _left_spawn_point_12 (CallFunction|SpawnLeftHall _current_spawn_point_28))
                  (CallFunction|SpawnMapPiece _left_spawn_point_12))
                (:then_1
                  (bind _current_spawn_point_29 (CallFunction|SpawnMapPiece _foward_spawn_point_7))
                  (bind _current_spawn_point_30 (CallFunction|SpawnMapPiece _current_spawn_point_29))
                  (bind _right_spawn_point_12 (CallFunction|SpawnRightTurn _current_spawn_point_30))
                  (bind _current_spawn_point_31 (CallFunction|SpawnMapPiece _right_spawn_point_12))
                  (bind _foward_spawn_point_11 (CallFunction|SpawnRightHall _current_spawn_point_31))
                  (bind _current_spawn_point_32 (CallFunction|SpawnMapPiece _foward_spawn_point_11))
                  (bind _right_spawn_point_13 (CallFunction|SpawnRightTurn _current_spawn_point_32))
                  (bind _left_spawn_point_13 (CallFunction|SpawnLeftTurn _right_spawn_point_13))
                  (bind _left_spawn_point_14 (CallFunction|SpawnLeftTurn _left_spawn_point_13))
                  (bind _right_spawn_point_14 (CallFunction|SpawnRightTurn _left_spawn_point_14))
                  (bind _right_spawn_point_15 (CallFunction|SpawnRightTurn _right_spawn_point_14))
                  (bind _left_spawn_point_15 (CallFunction|SpawnLeftTurn _right_spawn_point_15))
                  (bind _left_spawn_point_16 (CallFunction|SpawnLeftTurn _left_spawn_point_15))
                  (CallFunction|SpawnRightTurn _left_spawn_point_16))))))))))

(fn SpawnLeftHall
  (params (Spawn%20point :type Transform))
  (bind _returnvalue (Game|SpawnActorfromClass "/Game/Blueprints/Map_Pieces/Hall_Left.Hall_Left_C" Spawn%20point "Undefined" 0 0))
  (bind (_foward_spawn_point _left_spawn_point) (Default|GetHallSpawnPoints _returnvalue))
  (return _foward_spawn_point _left_spawn_point))

(fn SpawnRightHall
  (params (Spawn%20point :type Transform))
  (bind _returnvalue (Game|SpawnActorfromClass "/Game/Blueprints/Map_Pieces/Hall_Right.Hall_Right_C" Spawn%20point "Undefined" 0 0))
  (bind (_right_spawn_point _foward_spawn_point) (Default|GetHallSpawnPoints _returnvalue))
  (return _right_spawn_point _foward_spawn_point))

(fn Spawn3-way
  (params (Spawn%20point :type Transform))
  (bind _returnvalue (Game|SpawnActorfromClass "/Game/Blueprints/Map_Pieces/3-Way.3-Way_C" Spawn%20point "Undefined" 0 0))
  (bind (_left_spawn_point _right_spawn_point) (Default|Get3WaySpawnPoints _returnvalue))
  (return _left_spawn_point _right_spawn_point))

(fn Spawn4-way
  (params (Spawn%20point :type Transform))
  (bind _returnvalue (Game|SpawnActorfromClass "/Game/Blueprints/Map_Pieces/4-Way.4-Way_C" Spawn%20point "Undefined" 0 0))
  (bind (_left_spawn_point _right_spawn_point _foward_spawn_point) (Default|Get4WaySpawnPoints _returnvalue))
  (return _left_spawn_point _right_spawn_point _foward_spawn_point))

(fn SpawnLeftTurn
  (params (Spawn%20point :type Transform))
  (bind _returnvalue (Game|SpawnActorfromClass "/Game/Blueprints/Map_Pieces/Turn_Left.Turn_Left_C" Spawn%20point "Undefined" 0 0))
  (bind _spawnpoint (Default|GetSpawnPoint _returnvalue))
  (return _spawnpoint))

(fn SpawnRightTurn
  (params (Spawn%20point :type Transform))
  (bind _returnvalue (Game|SpawnActorfromClass "/Game/Blueprints/Map_Pieces/Turn_Right.Turn_Right_C" Spawn%20point "Undefined" 0 0))
  (bind _spawnpoint (Default|GetSpawnPoint _returnvalue))
  (return _spawnpoint))